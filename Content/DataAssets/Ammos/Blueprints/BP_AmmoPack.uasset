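; BP_AmmoPack is an ammo pickup actor that gives extra rounds to the player's current weapon.
; On BeginPlay it caches the first-person player character.
; Its PickUp event, when the player has a valid weapon, reads the round count from a data table row, adds it to the weapon via AddMaxPatrons, then destroys itself.
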(event EventPickUp
  (Utilities|IsValid (Variables|/Game/DataAssets/FirstPerson/Blueprints/BP_FirstPersonCharacter.BP_FirstPersonCharacter_C|GetWeapon (Variables|Default|GetPlayerCharacterInstance))
    (:Is%20Valid
      (bind _returnvalue (Utilities|GetDataTableRow (Variables|Default|GetDataTable) (Variables|Default|GetRowName))
        (:then
          (bind _output_get (Variables|Default|SetAmmoStructure _returnvalue))
          (bind _output_get_2 (Variables|Default|SetCountOfPatrons (Utilities|Struct|BreakS_AmmoStructure _output_get)))
          (Default|AddMaxPatrons (Variables|/Game/DataAssets/FirstPerson/Blueprints/BP_FirstPersonCharacter.BP_FirstPersonCharacter_C|GetWeapon (Variables|Default|GetPlayerCharacterInstance)) _output_get_2)
          (Actor|DestroyActor))))))

(event EventBeginPlay
  (bind _asbp_first_person_character (Utilities|Casting|CastToBP_FirstPersonCharacter (Game|GetPlayerCharacter 0)))
  (Variables|Default|SetPlayerCharacterInstance _asbp_first_person_character))

(fn ConstructionScript)